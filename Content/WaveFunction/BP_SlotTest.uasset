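; BP_SlotTest is a test actor for a wave function slot that shows a random module mesh.
; On BeginPlay it calls SetModule, which stores the given index but looks up a random row named 0 to 3 in DT_ModuleSet.
; When the row is found, its Module mesh is applied to the SM component.
; A separate SaySomething function prints the actor's location for debugging.
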(event `self.ReceiveBeginPlay`
  (`self.SetModule` 0))

(event `self.ReceiveActorBeginOverlap`
  (params (OtherActor :type "Actor Object Reference")))

(fn `SaySomething`
  (`KismetSystemLibrary.PrintString` (`KismetStringLibrary.Conv_VectorToString` (`self.K2_GetActorLocation`))))

(fn `SetModule`
  (params (ModuleIndex :type Integer))
  (set `self.ModuleIndex` ModuleIndex)
  (bind _returnvalue (`|GetDataTableRow` "/Game/WaveFunction/DT_ModuleSet.DT_ModuleSet" (`KismetStringLibrary.Conv_StringToName` (`KismetStringLibrary.Conv_IntToString` (`KismetMathLibrary.RandomIntegerInRange` 0 3))))
    (:`then`
      (`StaticMeshComponent.SetStaticMesh` (`self.SM`) (`.Module_8_46DF5F6C4E19DF3CA60315B3F95B36C3` (break `/Game/WaveFunction/ST_ModuleSet` _returnvalue))))))

(fn `UserConstructionScript`)