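; BP_InfiniteMap grows an endless 3D grid of BP_SlotTest actors around the player.
; BeginPlay seeds a cube of slots around the origin, stored in a map keyed by world position.
; Each tick it calls SaySomething on the player's slot, then spawns missing slots within PlayerVisionField.
; New slots are collected in TmpWorkSlotList, but CollapseChunk is an empty stub, so no wave-function collapse happens here.
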(event `self.ReceiveBeginPlay`
  (`|ExecutionSequence`
    (:`then_0`
      (for _index (range -9 10)
        (bind _output_get (set `self.x` _index))
        (for _index_2 (range -9 10)
          (bind _output_get_2 (set `self.y` _index_2))
          (for _index_3 (range -9 10)
            (bind _output_get_3 (set `self.z` _index_3))
            (bind _output_get_4 (set `self.TmpVector` (`KismetMathLibrary.MakeVector` (* _output_get (`self.SlotSize`)) (* _output_get_2 (`self.SlotSize`)) (* _output_get_3 (`self.SlotSize`)))))
            (`/Engine/EditorBlueprintResources/StandardMacros.IncrementInt` (`self.CurIndex`)
              (:`  `
                (bind _returnvalue (`|SpawnActorFromClass` "/Game/WaveFunction/BP_SlotTest.BP_SlotTest_C" (`KismetMathLibrary.MakeTransform` _output_get_4) "AdjustIfPossibleButAlwaysSpawn" "OverrideRootScale" null null))
                (`BlueprintMapLibrary.Map_Add` (`self.Map_V2Slot`) _output_get_4 _returnvalue)))))))))

(event `self.ReceiveTick`
  (params (DeltaSeconds :type "Float (single-precision)"))
  (`|ExecutionSequence`
    (:`then_0`
      (bind _asbp_slot_test (cast `/Game/WaveFunction/BP_SlotTest` (`BlueprintMapLibrary.Map_Find` (`self.Map_V2Slot`) (`self.PositionExchange` (`self.K2_GetActorLocation` (`GameplayStatics.GetPlayerPawn` 0))))))
      (`/Game/WaveFunction/BP_SlotTest.SaySomething` _asbp_slot_test))
    (:`then_1`
      (`self.Tick_SearchFields`))))

(fn `CollapseChunk`
  (params (WorkSlotList :type "Array of /Game/WaveFunction/BP_SlotTest Object Reference")))

(fn `GetTest`
  (for _index (range 10)
    (bind _output_get (set `self.x` _index))
    (for _index_2 (range 10)
      (bind _output_get_2 (set `self.y` _index_2))
      (for _index_3 (range 10)
        (bind _output_get_3 (set `self.z` _index_3))
        (bind _output_get_4 (set `self.TmpVector` (`KismetMathLibrary.MakeVector` (* _output_get (`self.SlotSize`)) (* _output_get_2 (`self.SlotSize`)) (* _output_get_3 (`self.SlotSize`)))))
        (bind _asbp_slot_test (cast `/Game/WaveFunction/BP_SlotTest` (`BlueprintMapLibrary.Map_Find` (`self.Map_V2Slot`) _output_get_4)))
        (`/Game/WaveFunction/BP_SlotTest.SaySomething` _asbp_slot_test)))))

(fn `PositionExchange`
  (params (Location :type "Vector Structure"))
  (returns (NewParam :type "Vector Structure"))
  (bind _slotsize (`self.SlotSize`))
  (bind _slotsize_2 (`self.SlotSize`))
  (bind _slotsize_3 (`self.SlotSize`))
  (return (`KismetMathLibrary.MakeVector` (* (/ (.x Location) _slotsize_2) _slotsize_2) (* (/ (.y Location) _slotsize) _slotsize) (* (/ (.z Location) _slotsize_3) _slotsize_3))))

(fn `Tick_SearchFields`
  (locals (LocalX :type Integer) (LocalY :type Integer) (LocalZ :type Integer) (LocalPlayerKoordinate :type "Vector Structure" :default (0.0 0.0 0.0)))
  (bind _returnvalue (+ (`KismetMathLibrary.MakeVector` (* (`self.SlotSize`) (`local.LocalX`)) (* (`self.SlotSize`) (`local.LocalY`)) (* (`self.SlotSize`) (`local.LocalZ`))) (`local.LocalPlayerKoordinate`)))
  (`KismetArrayLibrary.Array_Clear` (`self.TmpWorkSlotList`))
  (set `local.LocalPlayerKoordinate` (`self.PositionExchange` (`self.K2_GetActorLocation` (`GameplayStatics.GetPlayerPawn` 0))))
  (for _index (range (* (`self.PlayerVisionField`) -1) (+ (`self.PlayerVisionField`) 1))
    (set `local.LocalX` _index)
    (for _index_2 (range (* (`self.PlayerVisionField`) -1) (+ (`self.PlayerVisionField`) 1))
      (set `local.LocalY` _index_2)
      (for _index_3 (range (* (`self.PlayerVisionField`) -1) (+ (`self.PlayerVisionField`) 1))
        (set `local.LocalZ` _index_3)
        (if (not (`.ReturnValue` (`BlueprintMapLibrary.Map_Find` (`self.Map_V2Slot`) _returnvalue)))
          (bind _returnvalue_2 (`|SpawnActorFromClass` "/Game/WaveFunction/BP_SlotTest.BP_SlotTest_C" (`KismetMathLibrary.MakeTransform` _returnvalue) "AdjustIfPossibleButAlwaysSpawn" "OverrideRootScale" null null))
          (`BlueprintMapLibrary.Map_Add` (`self.Map_V2Slot`) _returnvalue _returnvalue_2)
          (`KismetArrayLibrary.Array_AddUnique` (`self.TmpWorkSlotList`) _returnvalue_2))))))

(fn `UserConstructionScript`)